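; Goal hole ("hoyo") trigger actor that wins the stage for the physics ball when its sphere is overlapped.
; On overlap it prints a debug message, looks up the first PhysicsBallBP in the level, sets StageWon and zeroes the ball's physics velocity.
; It zeroes velocity again if any component still reads positive.
; The overlapping actor is never checked, so any overlap triggers the win.
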(event `self.Sphere.OnComponentBeginOverlap`
  (params (OverlappedComponent :type "PrimitiveComponent Object Reference") (OtherActor :type "Actor Object Reference") (OtherComp :type "PrimitiveComponent Object Reference") (OtherBodyIndex :type Integer) (bFromSweep :type Boolean) (SweepResult :type "HitResult Structure (by ref)"))
  (`KismetSystemLibrary.PrintString` "hoyo!")
  (bind _outactors (`GameplayStatics.GetAllActorsOfClass` "/Game/RollingBP/Blueprints/PhysicsBallBP.PhysicsBallBP_C"))
  (bind _output (`|GetArrayItem` _outactors))
  (set `/Game/RollingBP/Blueprints/PhysicsBallBP.stage_won` true _output)
  (bind _ball (`/Game/RollingBP/Blueprints/PhysicsBallBP.Ball` _output))
  (`PrimitiveComponent.SetAllPhysicsLinearVelocity` _ball (0.0 0.0 0.0) false)
  (bind (_returnvalue_x _returnvalue_y _returnvalue_z) (`KismetMathLibrary.BreakVector` (`self.GetVelocity` _output)))
  (if (or (> _returnvalue_x 0.0) (> _returnvalue_y 0.0) (> _returnvalue_z 0.0))
    (`PrimitiveComponent.SetAllPhysicsLinearVelocity` _ball (0.0 0.0 0.0) false)))

(fn `UserConstructionScript`)